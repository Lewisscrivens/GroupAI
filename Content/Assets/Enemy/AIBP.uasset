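; Enemy AI Blueprint that stops the enemy from seeing the player while the player is hidden.
; BeginPlay caches the player character as a Player reference.
; Tick, throttled by a short Delay, polls the player's Hidden flag and, when set, turns off CanSeePlayer and clears the player-position Blackboard key.
; The graph only clears sight state and contains no detection logic that sets it.
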(event EventBeginPlay
  ;[1 1 1] Get the player
  (bind _asplayer (Utilities|Casting|CastToPlayer (Game|GetPlayerCharacter 0)))
  (Variables|Default|SetPlayer _asplayer))

(event EventTick
  (params (DeltaSeconds :type Float%20%28single-precision%29))
  ;[1 1 1] Ensure the ai cannot see the player when hidden.
  (Utilities|FlowControl|Delay 0.2)
  (if (Variables|/Script/GroupAI.GroupAICharacter|Gethidden (Variables|Default|GetPlayer))
    (Variables|Default|SetcanSeePlayer false)
    (AI|Components|Blackboard|ClearValue (AI|GetBlackboard 0) (Variables|Default|GetPlayerPosKey))))

(fn ConstructionScript)